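; Spawner that keeps a constant number of moving practice targets in the level, creating Count BP_PracticeTarget actors on BeginPlay.
; It binds each target's destroyed event to spawn a replacement and its reached-target event to assign a new move destination.
; Spawn points and destinations are random points within a horizontal radius and height band around the world origin, independent of the spawner's location.
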(event `self.ReceiveBeginPlay`
  (for _ (range 1 (+ (`self.Count`) 1))
    (`self.SpawnTarget`)))

(event `SpawnTarget`
  (bind _returnvalue (`|SpawnActorFromClass` "/Game/Logic/Misc/BP_PracticeTarget.BP_PracticeTarget_C" (`KismetMathLibrary.MakeTransform` (`self.GetRandomLocation`)) "AlwaysSpawn" "MultiplyWithRoot" null null))
  (add `self.OnDestroyed` _returnvalue (delegate `OnTargetDestroyed`))
  (add `BzPracticeTarget.OnReachedTarget` _returnvalue (delegate `SetNewTarget`))
  (`self.SetNewTarget` _returnvalue))

(event `OnTargetDestroyed` :!signature `self.OnDestroyed`
  (params (DestroyedActor :type "Actor Object Reference"))
  (`self.SpawnTarget`))

(event `SetNewTarget`
  (params (Sender :type "BzPracticeTarget Object Reference"))
  (`BzPracticeTarget.SetMoveTarget` Sender (`self.GetRandomLocation`)))

(fn `GetRandomLocation`
  (returns (location :type "Vector Structure"))
  (return (+ (* (`KismetMathLibrary.Conv_RotatorToVector` (`KismetMathLibrary.MakeRotator` 0.0 0.0 (`KismetMathLibrary.RandomFloatInRange` 0.0 360.0))) (`KismetMathLibrary.RandomFloatInRange` 0.0 4000.0)) (`KismetMathLibrary.MakeVector` 0.0 0.0 (`KismetMathLibrary.RandomFloatInRange` 450.0 600.0)))))

(fn `UserConstructionScript`)