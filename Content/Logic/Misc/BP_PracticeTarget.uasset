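; BP_PracticeTarget is a destructible practice target that shows its health through colored indicators.
; On each health state change, two indicator meshes switch emissive materials from red to green by health quadrant.
; When the BzHealth component reports death, it spawns an enlarged projectile-hit Niagara effect and destroys itself.
; A timeline started on BeginPlay animates the root component's scale.
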(event `self.BzHealth.OnStateChanged`
  (params (Sender :type "BzHealthComponent Object Reference"))
  (if (`BzHealthComponent.IsAlive` Sender)
    (`PrimitiveComponent.SetMaterial` (`self.HealthIndicator`) 0 (select `int` (`BzHealthComponent.GetHealthQuadrant` Sender) :`0` "/Game/Art/Materials/MI_Emissive_Red.MI_Emissive_Red" :`1` "/Game/Art/Materials/MI_EmissiveOrange.MI_EmissiveOrange" :`2` "/Game/Art/Materials/MI_Emissive_Yellow.MI_Emissive_Yellow" :`3` "/Game/Art/Materials/MI_Emissive_Green.MI_Emissive_Green" :!type "MaterialInterface Object Reference"))
    (`PrimitiveComponent.SetMaterial` (`self.HealthIndicator1`) 0 (select `int` (`BzHealthComponent.GetHealthQuadrant` Sender) :`0` "/Game/Art/Materials/MI_Emissive_Red.MI_Emissive_Red" :`1` "/Game/Art/Materials/MI_EmissiveOrange.MI_EmissiveOrange" :`2` "/Game/Art/Materials/MI_Emissive_Yellow.MI_Emissive_Yellow" :`3` "/Game/Art/Materials/MI_Emissive_Green.MI_Emissive_Green" :!type "MaterialInterface Object Reference"))
    (else
      (bind _returnvalue (`NiagaraFunctionLibrary.SpawnSystemAtLocation` "/Game/Vfx/NS_ProjectileHit.NS_ProjectileHit" (`self.K2_GetActorLocation`)))
      (`NiagaraComponent.SetVariableFloat` _returnvalue "RadiusCoef" 2.0)
      (`self.K2_DestroyActor`))))

(event `self.ReceiveBeginPlay`
  (bind (_direction _scale) (`Timeline|Timeline`)
    (:`Update`
      (`SceneComponent.SetRelativeScale3D` (`self.RootComponent`) (`KismetMathLibrary.Conv_DoubleToVector` _scale)))))

(fn `UserConstructionScript`)