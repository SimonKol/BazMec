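; BP_EdgeWalls is an actor that forms a square enclosure from four wall components: North, East, South and West.
; The construction script derives each wall's transform from Side and Height, offsetting by half the side, raising by half the height, rotating and scaling at one-hundredth of those dimensions.
; On BeginPlay, the actor hides itself in game unless Visible is set, so it can serve as an invisible boundary.
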(event EventBeginPlay
  (Rendering|SetActorHiddenInGame (not (Variables|_Bz|GetVisible))))

(fn ConstructionScript
  (bind _returnvalue (|({20EBC52E-43DE-B456-1BDA-95961F554E20}*0.010000)))
  (bind _returnvalue_2 (|({FA5E5D21-4EB7-BB40-3535-FBB9FDE7A201}*0.010000)))
  (bind _returnvalue_3 (|({20EBC52E-43DE-B456-1BDA-95961F554E20}*0.500000)))
  (bind _returnvalue_4 (|({FA5E5D21-4EB7-BB40-3535-FBB9FDE7A201}*0.500000)))
  (bind _returnvalue_5 (* _returnvalue_3 -1.0))
  (Transformation|SetRelativeTransform (Variables|Default|GetNorth) (Math|Transform|MakeTransform (Math|Vector|MakeVector _returnvalue_3 0.0 _returnvalue_4) "90.000000,0.000000,0.000000" (Math|Vector|MakeVector _returnvalue_2 _returnvalue 1.0)) false false)
  (Transformation|SetRelativeTransform (Variables|Default|GetEast) (Math|Transform|MakeTransform (Math|Vector|MakeVector 0.0 _returnvalue_3 _returnvalue_4) "0.000000,0.000000,-90.000000" (Math|Vector|MakeVector _returnvalue _returnvalue_2 1.0)) false false)
  (Transformation|SetRelativeTransform (Variables|Default|GetSouth) (Math|Transform|MakeTransform (Math|Vector|MakeVector _returnvalue_5 0.0 _returnvalue_4) "-90.000000,0.000000,0.000000" (Math|Vector|MakeVector _returnvalue_2 _returnvalue 1.0)) false false)
  (Transformation|SetRelativeTransform (Variables|Default|GetWest) (Math|Transform|MakeTransform (Math|Vector|MakeVector 0.0 _returnvalue_5 _returnvalue_4) "0.000000,0.000000,90.000000" (Math|Vector|MakeVector _returnvalue _returnvalue_2 1.0)) false false))