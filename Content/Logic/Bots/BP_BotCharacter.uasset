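; BP_BotCharacter is an enemy-style bot character that spawns with a random weapon and breaks apart when killed.
; On BeginPlay its WeaponComponent spawns a mini cannon, or occasionally a mini rocket launcher, snapped to the AimPoint.
; HealthComponent state changes recolor an emissive health indicator by health quadrant, or trigger OnDeath.
; Death disables the radar, breaks the indicator, turns off capsule and hitbox collision, and detaches meshes as physics debris.
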(event `self.ReceiveBeginPlay`
  (bind _returnvalue (`BzWeaponComponent.SpawnWeapon` (`self.WeaponComponent`) (select `bool` (> (`KismetMathLibrary.RandomFloat`) 0.87) :`false` "/Game/Logic/Weapons/BP_W_MiniCannon.BP_W_MiniCannon_C" :`true` "/Game/Logic/Weapons/BP_W_MiniRocketLauncher.BP_W_MiniRocketLauncher_C" :!type "BzWeapon Class Reference")))
  (`self.K2_AttachToComponent` _returnvalue (`self.AimPoint`) "None" "SnapToTarget" "SnapToTarget" "SnapToTarget" true))

(event `self.HealthComponent.OnStateChanged`
  (params (Sender :type "BzHealthComponent Object Reference"))
  (if (`BzHealthComponent.IsAlive` Sender)
    (`self.UpdateHealthIndicator` (`BzHealthComponent.GetHealthQuadrant` Sender))
    (else
      (`self.OnDeath`))))

(fn `OnDeath`
  (bind _capsulecomponent (`self.CapsuleComponent`))
  (`|ExecutionSequence`
    (:`then_0`
      (`BzRadarComponent.SetEnabled` (`self.BzRadar`) false))
    (:`then_1`
      (`PrimitiveComponent.SetMaterial` (`self.HealthIndicator`) 0 "/Game/Art/Materials/M_BrokenHealthIndicator.M_BrokenHealthIndicator")
      (`PrimitiveComponent.SetCollisionEnabled` _capsulecomponent "NoCollision")
      (`PrimitiveComponent.SetCollisionEnabled` (`self.HitBox`) "NoCollision")
      (bind _children (`SceneComponent.GetChildrenComponents` _capsulecomponent true))
      (for _array_element _children
        (bind _asmesh_component (cast `MeshComponent` _array_element))
        (`SceneComponent.K2_DetachFromComponent` _asmesh_component "KeepRelative" "KeepRelative" "KeepRelative" true)
        (`PrimitiveComponent.SetCollisionResponseToChannel` _asmesh_component "ECC_Pawn" "ECR_Ignore")
        (`PrimitiveComponent.SetSimulatePhysics` _asmesh_component true)))))

(fn `UpdateHealthIndicator`
  (params (quadrant :type Integer))
  (`PrimitiveComponent.SetMaterial` (`self.HealthIndicator`) 0 (select `int` quadrant :`0` "/Game/Art/Materials/MI_Emissive_Red.MI_Emissive_Red" :`1` "/Game/Art/Materials/MI_EmissiveOrange.MI_EmissiveOrange" :`2` "/Game/Art/Materials/MI_Emissive_Yellow.MI_Emissive_Yellow" :`3` "/Game/Art/Materials/MI_Emissive_Cyan.MI_Emissive_Cyan" :!type "MaterialInterface Object Reference")))

(fn `UserConstructionScript`
  (`self.UpdateHealthIndicator` 3))