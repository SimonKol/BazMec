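; BP_Projectile_Rocket is a rocket projectile that supplies the visuals for launch, impact and end of flight.
; Start activates the exhaust effect and shows the cone, while impact spawns an enlarged Niagara hit effect tinted with the projectile's color.
; Finish hides the cone and deactivates the exhaust, then waits a few seconds before calling ConfirmRelease, delaying the projectile's release.
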(event `self.BP_OnImpact`
  (params (Hit :type "HitResult Structure (by ref)"))
  (bind _returnvalue (`NiagaraFunctionLibrary.SpawnSystemAtLocation` "/Game/Vfx/NS_ProjectileHit.NS_ProjectileHit" (`.ImpactPoint` (`GameplayStatics.BreakHitResult` Hit)) (struct) (10.0 10.0 10.0)))
  (`NiagaraComponent.SetVariableFloat` _returnvalue "RadiusCoef" 10.0)
  (`NiagaraComponent.SetVariableLinearColor` _returnvalue "Color" (`self.Color`)))

(event `self.BP_OnStarted`
  (params (Location :type "Vector Structure (by ref)") (Rotation :type "Rotator Structure (by ref)"))
  (`ActorComponent.Activate` (`self.Exhaust`) true)
  (`SceneComponent.SetVisibility` (`self.Cone`) true false))

(event `self.BP_OnFinished`
  (`SceneComponent.SetVisibility` (`self.Cone`) false false)
  (`ActorComponent.Deactivate` (`self.Exhaust`))
  (`KismetSystemLibrary.Delay` 5.0)
  (`self.ConfirmRelease`))

(fn `UserConstructionScript`)