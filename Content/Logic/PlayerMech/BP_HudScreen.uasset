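; BP_HudScreen is an in-world screen actor that shows mech HUD content through a 3D widget component.
; SetContent passes a given widget and mech to the WBP_DisplaySlot hosted by that component, doing nothing if the cast fails.
; On construction, SyncSizeAndResolution sets the draw size from ScreenResolution and scales the component so the screen's world size matches ScreenSize independently of pixel resolution.
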(fn `SetContent`
  (params (widget :type "BzMechWidget Soft Class Reference") (mech :type "BzPlayerMech Object Reference"))
  (bind _aswbp_display_slot (cast `/Game/UI/Player/WBP_DisplaySlot` (`WidgetComponent.GetUserWidgetObject` (`self.Widget3d`))))
  (`/Game/UI/Player/WBP_DisplaySlot.SetContent` _aswbp_display_slot widget mech))

(fn `SyncSizeAndResolution`
  (bind (_x _y) (`KismetMathLibrary.BreakVector2D` (/ (`self.ScreenSize`) (`self.ScreenResolution`))))
  (`WidgetComponent.SetDrawSize` (`self.Widget3d`) (`self.ScreenResolution`))
  (`SceneComponent.SetRelativeScale3D` (`self.Widget3d`) (`KismetMathLibrary.MakeVector` 1.0 _x _y)))

(fn `UserConstructionScript`
  (`self.SyncSizeAndResolution`))