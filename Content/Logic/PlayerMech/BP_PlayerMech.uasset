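; BP_PlayerMech is the player-controlled mech, handling move, look, jump and speed boost input.
; On BeginPlay it spawns three HUD screen actors in an arc under DisplayRoot, showing weapons, center and radar widgets bound to the mech.
; When its health component reports death, it disables input and releases both weapon triggers.
; Weapon fire starts a camera shake.
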(event `self.ReceiveBeginPlay`
  (`self.MakeDisplays`))

(event `self.HealthComponent.OnStateChanged`
  (params (Sender :type "BzHealthComponent Object Reference"))
  (if (not (`BzHealthComponent.IsAlive` Sender))
    (bind _asplayer_controller (cast `PlayerController` (`self.GetController`)))
    (`self.DisableInput` _asplayer_controller)
    (`BzWeapon.SetTriggerState` (`self.GetPrimaryWeapon`) false)
    (`BzWeapon.SetTriggerState` (`self.GetSecondaryWeapon`) false)))

(event `self.BP_OnWeaponFired`
  (`CameraShakeSourceComponent.StartCameraShake` :`self` (`self.CamShakeSource`) :`InCameraShake` "/Game/Logic/PlayerMech/BP_WeaponFiredCamShake.BP_WeaponFiredCamShake_C"))

(event `EnhancedInput|/Game/Input/IA_Move`
  (params (ActionValue :type "Vector2D Structure") (ElapsedSeconds :type "Float (double-precision)") (TriggeredSeconds :type "Float (double-precision)") (InputAction :type "InputAction Object Reference" :default "/Game/Input/IA_Move.IA_Move"))
  (bind (_x _y) (`KismetMathLibrary.BreakVector2D` ActionValue))
  (bind (_returnvalue_roll _returnvalue_pitch _returnvalue_yaw) (`KismetMathLibrary.BreakRotator` (`self.GetControlRotation`)))
  (:`Triggered`
    (`self.AddMovementInput` (`KismetMathLibrary.GreaterGreater_VectorRotator` (`KismetMathLibrary.MakeVector` _y _x) (`KismetMathLibrary.MakeRotator` 0.0 0.0 _returnvalue_yaw)))))

(event `EnhancedInput|/Game/Input/IA_MouseLook`
  (params (ActionValue :type "Vector2D Structure") (ElapsedSeconds :type "Float (double-precision)") (TriggeredSeconds :type "Float (double-precision)") (InputAction :type "InputAction Object Reference" :default "/Game/Input/IA_MouseLook.IA_MouseLook"))
  (bind (_x _y) (`KismetMathLibrary.BreakVector2D` ActionValue))
  (:`Triggered`
    (`self.AddControllerYawInput` _x)
    (`self.AddControllerPitchInput` _y)))

(event `EnhancedInput|/Game/Input/IA_Jump`
  (params (ActionValue :type Boolean) (ElapsedSeconds :type "Float (double-precision)") (TriggeredSeconds :type "Float (double-precision)") (InputAction :type "InputAction Object Reference" :default "/Game/Input/IA_Jump.IA_Jump"))
  (:`Started`
    (`self.TryJump`)))

(event `EnhancedInput|/Game/Input/IA_SpeedBoost`
  (params (ActionValue :type Boolean) (ElapsedSeconds :type "Float (double-precision)") (TriggeredSeconds :type "Float (double-precision)") (InputAction :type "InputAction Object Reference" :default "/Game/Input/IA_SpeedBoost.IA_SpeedBoost"))
  (:`Started`
    (`self.TrySpeedBoost`)))

(fn `MakeDisplay`
  (params (Angle :type "Float (double-precision)") (widget :type "BzMechWidget Soft Class Reference"))
  (bind _returnvalue (`|SpawnActorFromClass` "/Game/Logic/PlayerMech/BP_HudScreen.BP_HudScreen_C" (`KismetMathLibrary.MakeTransform` (0.0 0.0 0.0)) "AlwaysSpawn" "MultiplyWithRoot" null null))
  (`self.K2_AttachToComponent` _returnvalue (`self.DisplayRoot`) "None" "SnapToTarget" "SnapToTarget" "KeepRelative" true)
  (`self.K2_SetActorRelativeTransform` _returnvalue (`KismetMathLibrary.MakeTransform` (`KismetMathLibrary.GreaterGreater_VectorRotator` (55.0 0.0 -15.0) (`KismetMathLibrary.MakeRotator` 0.0 0.0 Angle)) (`KismetMathLibrary.ComposeRotators` (`KismetMathLibrary.MakeRotator` 0.0 15.0) (`KismetMathLibrary.MakeRotator` 0.0 0.0 (+ Angle 180.0)))) false false)
  (`/Game/Logic/PlayerMech/BP_HudScreen.SetContent` _returnvalue widget self))

(fn `MakeDisplays`
  (`self.MakeDisplay` -30.0 "/Game/UI/Player/WBP_Display_Weapons.WBP_Display_Weapons_C")
  (`self.MakeDisplay` 0.0 "/Game/UI/Player/WBP_Display_Center.WBP_Display_Center_C")
  (`self.MakeDisplay` 30.0 "/Game/UI/Player/WBP_Display_Radar.WBP_Display_Radar_C"))

(fn `UserConstructionScript`)