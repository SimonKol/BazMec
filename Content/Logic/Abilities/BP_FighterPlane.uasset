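; BP_FighterPlane is an ability actor for a fighter plane that flies over and launches a rocket strike at a target.
; Tick moves it straight along its forward vector at Speed, without sweeping for collision.
; On BeginPlay it waits a short random delay, then spawns a StrikeRocket through the Bz projectile subsystem, aimed from its current location toward StrikeTarget with itself as shooter.
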(event `self.ReceiveBeginPlay`
  (bind _returnvalue (`self.K2_GetActorLocation`))
  (bind _returnvalue_2 (subsystem `BzProjectileSubsystem`))
  (`KismetSystemLibrary.Delay` (`KismetMathLibrary.RandomFloatInRange` 6.0 7.0))
  (bind _result (`BzProjectileSubsystem.TryGetProjectileType` _returnvalue_2 "StrikeRocket"))
  (`BzProjectileSubsystem.NewProjectile` _returnvalue_2 _result _returnvalue (`KismetMathLibrary.Normal` (- (`self.StrikeTarget`) _returnvalue)) self))

(event `self.ReceiveTick`
  (params (DeltaSeconds :type "Float (single-precision)"))
  (`self.K2_AddActorWorldOffset` (* (`self.GetActorForwardVector`) (* DeltaSeconds (`self.Speed`)))))

(fn `UserConstructionScript`)