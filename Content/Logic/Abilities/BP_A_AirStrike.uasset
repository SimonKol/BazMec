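; Air strike ability that calls in a fighter plane on the impact point of the hit it is executed with.
; SpawnJet picks a random heading, then spawns BP_FighterPlane high above and far behind the target along that heading, passing it the strike target.
; A colored decal marks the target, and both decal and plane expire on fixed lifespans.
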(event `self.Execute`
  (params (Params :type "BzStartAbilityParams Structure (by ref)"))
  (`self.SpawnJet` (`.ImpactPoint` (`GameplayStatics.BreakHitResult` (`.Hit` (break `BzStartAbilityParams` Params))))))

(fn `SpawnJet`
  (params (target :type "Vector Structure"))
  (locals (dir :type "Rotator Structure") (spawnPoint :type "Vector Structure") (decalColor :type "LinearColor Structure" :default (struct :`R` 20.0 :`G` 1.0 :`B` 1.0)))
  (bind _output_get (set `local.dir` (`KismetMathLibrary.MakeRotator` 0.0 0.0 (`KismetMathLibrary.RandomFloatInRange` 0.0 360.0))))
  (set `local.spawnPoint` (+ target (`KismetMathLibrary.MakeVector` 0.0 0.0 (* (`KismetMathLibrary.RandomFloatInRange` 400.0 500.0) 100.0)) (* (`KismetMathLibrary.Conv_RotatorToVector` _output_get) -200000.0)))
  (`|ExecutionSequence`
    (:`then_0`
      (bind _returnvalue (`GameplayStatics.SpawnDecalAtLocation` "/Game/Art/Materials/M_StrikeTargetDecal.M_StrikeTargetDecal" (500.0 500.0 500.0) (`local.target`) (struct :`Pitch` -90.0) 8.0))
      (`DecalComponent.SetDecalColor` _returnvalue (`local.decalColor`)))
    (:`then_1`
      (bind _returnvalue_2 (`|SpawnActorFromClass` "/Game/Logic/Abilities/BP_FighterPlane.BP_FighterPlane_C" (`KismetMathLibrary.MakeTransform` (`local.spawnPoint`) (`local.dir`)) "Undefined" "MultiplyWithRoot" null (`local.target`) null))
      (`Actor.SetLifeSpan` _returnvalue_2 20.0))))