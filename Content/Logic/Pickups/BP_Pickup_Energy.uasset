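; BP_Pickup_Energy is a pickup that restores energy to the user who collects it.
; CanPickup allows collection only when the object obtained from the user through Get is valid and reports NeedsRestore, otherwise returning false.
; On DoPickup it validates that same object and calls Restore with the Energy value.
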(event `self.DoPickup`
  (params (User :type "Actor Object Reference"))
  (bind _returnvalue (`BzEnergyComponent.Get` User))
  (`/Engine/EditorBlueprintResources/StandardMacros.IsValid` _returnvalue
    (:`Is Valid`
      (`BzEnergyComponent.Restore` _returnvalue (`self.Energy`)))))

(fn `CanPickup`
  (params (User :type "Actor Object Reference"))
  (returns (ReturnValue :type Boolean))
  (`|ExecutionSequence`
    (:`then_0`
      (bind _returnvalue (`BzEnergyComponent.Get` User))
      (`/Engine/EditorBlueprintResources/StandardMacros.IsValid` _returnvalue
        (:`Is Valid`
          (return (`BzEnergyComponent.NeedsRestore` _returnvalue)))))
    (:`then_1`
      (return false))))

(fn `UserConstructionScript`)